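; BP_GameManager is a game manager that handles the level-complete screen and fade transitions into and out of levels.
; It creates a hidden win widget at BeginPlay, then OnFinishLevel shows it and switches input to UI only.
; While a transition flag is set, Tick lerps the camera gain between zero and one by timer progress and copies it through the player's post-process component to its camera.
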(event `self.OnBeginPlay`
  (bind _returnvalue (`|CreateWidget` "/Game/Blueprints/Widgets/WinWidget.WinWidget_C"))
  (bind _output_get (set `self.WinCanvas` _returnvalue))
  (`UserWidget.AddToViewport` _output_get 10)
  (`Widget.SetVisibility` _output_get "Hidden"))

(event `self.OnFinishLevel`
  (bind _wincanvas (`self.WinCanvas`))
  (`Widget.SetVisibility` _wincanvas "Visible")
  (`WidgetBlueprintLibrary.SetInputMode_UIOnlyEx` (`GameplayStatics.GetPlayerController` 0) _wincanvas))

(event `self.OnTick`
  (params (deltaTime :type "Float (single-precision)"))
  (bind _returnvalue (`KismetMathLibrary.Lerp` 1.0 0.0 (* (`self.levelTransitionTimer`) (/ 1.0 (`self.levelTransitionTime`)))))
  (bind _returnvalue_2 (`KismetMathLibrary.Lerp` 0.0 1.0 (* (`self.levelTransitionTimer`) (/ 1.0 (`self.levelTransitionTime`)))))
  (if (`self.transitionIntoLevel`)
    (`KismetMathLibrary.Vector4_Set` (`self.Camera Gain`) _returnvalue_2 _returnvalue_2 _returnvalue_2 _returnvalue_2)
    (bind _output_get (set `PostProcessComponent.Settings` (make `PostProcessSettings` :`ColorGain` (`self.Camera Gain`)) (`PawnBase.postProcessComponent` (`self.playerRef`)) :!label _label))
    (set `CameraComponent.PostProcessSettings` _output_get (`PawnBase.cameraComponent` (`self.playerRef`)))
    (elif (`self.transitionOutOfLevel`)
      (`KismetMathLibrary.Vector4_Set` (`self.Camera Gain`) _returnvalue _returnvalue _returnvalue _returnvalue)
      (goto _label))))