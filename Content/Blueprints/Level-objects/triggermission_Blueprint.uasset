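; Mission trigger actor that lets the player open a level select menu while standing inside it.
; On BeginPlay it enables input and adds a hidden Level_select widget to the viewport.
; Overlap with BP_Parasite sets a flag that lets the E key toggle the widget's visibility through a FlipFlop.
; Leaving the trigger clears the flag and hides the widget without resetting the FlipFlop.
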(event `self.ReceiveBeginPlay`
  (`self.EnableInput` (`GameplayStatics.GetPlayerController` 0))
  (bind _returnvalue (`|CreateWidget` "/Game/Blueprints/Widgets/level_select.level_select_C"))
  (`UserWidget.AddToViewport` _returnvalue 0)
  (`Widget.SetVisibility` _returnvalue "Hidden"))

(event `self.ReceiveActorBeginOverlap`
  (params (OtherActor :type "Actor Object Reference"))
  (cast `/Game/Blueprints/Characters/BP_Parasite` OtherActor)
  (set `self.enable_missionbool` true))

(event `self.ReceiveActorEndOverlap`
  (params (OtherActor :type "Actor Object Reference"))
  (cast `/Game/Blueprints/Characters/BP_Parasite` OtherActor)
  (set `self.enable_missionbool` false)
  (`Widget.SetVisibility` (stale `self.ReceiveBeginPlay` _returnvalue) "Hidden"))

(event `Key|E`
  (params (Key :type "Key Structure"))
  (:`Pressed`
    (if (`self.enable_missionbool`)
      (`/Engine/EditorBlueprintResources/StandardMacros.FlipFlop`
        (:`A`
          (`Widget.SetVisibility` (stale `self.ReceiveBeginPlay` _returnvalue) "Visible"))
        (:`B`
          (`Widget.SetVisibility` (stale `self.ReceiveBeginPlay` _returnvalue) "Hidden"))))))

(fn `UserConstructionScript`)