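; Swinging door actor that opens once when something overlaps its front or back collision, and knocks back enemies caught while it opens.
; A timeline rotates the pivot from its initial yaw using a front or back curve, chosen by the side triggered.
; Overlap events are toggled on trigger, and melee or shooter enemies overlapping afterward receive knockback.
; When the timeline finishes, a sound plays and both collisions stop generating overlaps.
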(event `self.ReceiveBeginPlay`
  (bind (_returnvalue_roll _returnvalue_pitch _returnvalue_yaw) (`KismetMathLibrary.BreakRotator` (`SceneComponent.K2_GetComponentRotation` (`self.RotationPoint`))))
  (set `self.Z-rot` _returnvalue_yaw))

(event `self.FrontCollision.OnComponentBeginOverlap`
  (params (OverlappedComponent :type "PrimitiveComponent Object Reference") (OtherActor :type "Actor Object Reference") (OtherComp :type "PrimitiveComponent Object Reference") (OtherBodyIndex :type Integer) (bFromSweep :type Boolean) (SweepResult :type "HitResult Structure (by ref)"))
  (bind _returnvalue (`self.K2_GetActorLocation`))
  (if (`self.IsOpening`)
    (bind _asbp_enemy_melee (cast `/Game/Blueprints/Characters/AI/Melee/BP_Enemy_Melee` OtherActor)
      (:`then`
        (bind _regretfullchild (`/Game/Blueprints/Characters/AI/Melee/BP_Enemy_Melee.RegretfullChild` _asbp_enemy_melee))
        (set `/Game/Blueprints/Characters/AllEnemy_Component.KnockbackVector` _returnvalue _regretfullchild)
        (`/Game/Blueprints/Characters/AllEnemy_Component.EnemyKnockback` _regretfullchild))
      (:`CastFailed`
        (bind _asbp_enemy_shooter (cast `/Game/Blueprints/Characters/AI/Shooter/BP_Enemy_Shooter` OtherActor))
        (bind _regretfullchild_2 (`/Game/Blueprints/Characters/AI/Shooter/BP_Enemy_Shooter.RegretfullChild` _asbp_enemy_shooter))
        (set `/Game/Blueprints/Characters/AllEnemy_Component.KnockbackVector` _returnvalue _regretfullchild_2)
        (`/Game/Blueprints/Characters/AllEnemy_Component.EnemyKnockback` _regretfullchild_2)))
    (else
      (set `self.DoorOpener` OtherActor)
      (`self.Change- Overlap-function` false)
      (`self.Change- Overlap-function` true)
      (set `self.IsOpening` true)
      (set `self.IsFront` true)
      (bind (_direction _frontopen _backopen) (`Timeline|OpeningTimeline` :!label _label)
        (:`Update`
          (if (`self.IsFront`)
            (`SceneComponent.K2_SetWorldRotation` (`self.RotationPoint`) (`KismetMathLibrary.MakeRotator` 0.0 0.0 (+ _frontopen (`self.Z-rot`))) false true)
            (else
              (`SceneComponent.K2_SetWorldRotation` (`self.RotationPoint`) (`KismetMathLibrary.MakeRotator` 0.0 0.0 (+ _backopen (`self.Z-rot`))) false true))))
        (:`Finished`
          (`GameplayStatics.PlaySoundAtLocation` (`self.DoorSound`) (`SceneComponent.K2_GetComponentLocation` (`self.Door`)) (struct) 1.0 1.0 0.0 null null null)
          (`self.Change- Overlap-function` false))))))

(event `self.BackCollision.OnComponentBeginOverlap`
  (params (OverlappedComponent :type "PrimitiveComponent Object Reference") (OtherActor :type "Actor Object Reference") (OtherComp :type "PrimitiveComponent Object Reference") (OtherBodyIndex :type Integer) (bFromSweep :type Boolean) (SweepResult :type "HitResult Structure (by ref)"))
  (bind _returnvalue (`self.K2_GetActorLocation`))
  (if (`self.IsOpening`)
    ;[1 1 1] Knockback
    (bind _asbp_enemy_melee (cast `/Game/Blueprints/Characters/AI/Melee/BP_Enemy_Melee` OtherActor)
      (:`then`
        (bind _regretfullchild (`/Game/Blueprints/Characters/AI/Melee/BP_Enemy_Melee.RegretfullChild` _asbp_enemy_melee))
        (set `/Game/Blueprints/Characters/AllEnemy_Component.KnockbackVector` _returnvalue _regretfullchild)
        (`/Game/Blueprints/Characters/AllEnemy_Component.EnemyKnockback` _regretfullchild))
      (:`CastFailed`
        (bind _asbp_enemy_shooter (cast `/Game/Blueprints/Characters/AI/Shooter/BP_Enemy_Shooter` OtherActor))
        (bind _regretfullchild_2 (`/Game/Blueprints/Characters/AI/Shooter/BP_Enemy_Shooter.RegretfullChild` _asbp_enemy_shooter))
        (set `/Game/Blueprints/Characters/AllEnemy_Component.KnockbackVector` _returnvalue _regretfullchild_2)
        (`/Game/Blueprints/Characters/AllEnemy_Component.EnemyKnockback` _regretfullchild_2)))
    (else
      (set `self.DoorOpener` OtherActor)
      (`self.Change- Overlap-function` false)
      (`self.Change- Overlap-function` true)
      (set `self.IsOpening` true)
      (set `self.IsFront` false)
      (goto _label))))

(fn `Change- Overlap-function`
  (params (`On-Off` :type Boolean))
  (bind _output_get (set `PrimitiveComponent.bGenerateOverlapEvents` `On-Off` (`self.FrontCollision`)))
  (set `PrimitiveComponent.bGenerateOverlapEvents` _output_get (`self.BackCollision`)))

(fn `UserConstructionScript`)