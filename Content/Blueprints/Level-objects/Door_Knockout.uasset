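; Door that shooter and melee enemies swing open from either side, stunning shooter enemies that hit its push boxes.
; Front and back trigger boxes drive the DoorOpen timeline, reversing through closed when direction changes, and Tick applies the yaw to RotationPoint.
; Push boxes activate while the door is pushed and call Doorstun with a knockback vector based on CenterPoint.
; A completed swing destroys both triggers, leaving the door open.
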(event `self.ReceiveBeginPlay`
  (bind (_returnvalue_roll _returnvalue_pitch _returnvalue_yaw) (`KismetMathLibrary.BreakRotator` (`SceneComponent.K2_GetComponentRotation` (`self.Rotation point`))))
  (bind _output_get (set `self.Y-rot` _returnvalue_yaw))
  (set `self.Start-Y-rot` _output_get)
  (`self.Push-off`))

(event `self.ReceiveTick`
  (params (DeltaSeconds :type "Float (single-precision)"))
  (`SceneComponent.K2_SetWorldRotation` (`self.Rotation point`) (`KismetMathLibrary.MakeRotator` 0.0 0.0 (`self.Y-rot`)) false true))

(event `EnemyStunned`)

(event `self.MoveCollision-front.OnComponentBeginOverlap`
  (params (OverlappedComponent :type "PrimitiveComponent Object Reference") (OtherActor :type "Actor Object Reference") (OtherComp :type "PrimitiveComponent Object Reference") (OtherBodyIndex :type Integer) (bFromSweep :type Boolean) (SweepResult :type "HitResult Structure (by ref)"))
  (cast `/Game/Blueprints/Characters/AI/Shooter/BP_Enemy_Shooter` OtherActor
    (:`then`
      _)
    (:`CastFailed`
      (cast `/Game/Blueprints/Characters/AI/Melee/BP_Enemy_Melee` OtherActor)))
  (set `PrimitiveComponent.bGenerateOverlapEvents` false (`self.MoveCollision-back`))
  (`self.Push-on`)
  (if (`self.Closing`)
    (if (`self.BackSide`)
      (set `self.Reversing` true :!label _label)
      ;[1 1 1] Spaghett
      (bind (_direction _opening) (`Timeline|DoorOpen` :!via `Reverse` :!label _label_2)
        (:`Update`
          (if (`self.BackSide`)
            (set `self.Y-rot` (+ (* _opening -1.0) (`self.Start-Y-rot`)))
            (else
              (set `self.Y-rot` (+ _opening (`self.Start-Y-rot`))))))
        (:`Finished`
          (if (`self.Reversing`)
            (set `self.Reversing` false)
            (set `self.Closing` false)
            (if (`self.BackSide`)
              (set `self.BackSide` false)
              (goto _label_2)
              (else
                (set `self.BackSide` true)
                (goto _label_2)))
            (else
              (`ActorComponent.K2_DestroyComponent` (`self.MoveCollision-back`))
              (`ActorComponent.K2_DestroyComponent` (`self.MoveCollision-front`))))))
      (else
        (goto _label_2)))
    (else
      (set `self.Closing` (!= (`self.Y-rot`) (`self.Start-Y-rot`)))
      (set `self.BackSide` false)
      (goto _label_2))))

(event `self.MoveCollision-front.OnComponentEndOverlap`
  (params (OverlappedComponent :type "PrimitiveComponent Object Reference") (OtherActor :type "Actor Object Reference") (OtherComp :type "PrimitiveComponent Object Reference") (OtherBodyIndex :type Integer))
  (bind _movecollision_back (`self.MoveCollision-back`))
  (cast `/Game/Blueprints/Characters/AI/Shooter/BP_Enemy_Shooter` OtherActor
    (:`then`
      _)
    (:`CastFailed`
      (cast `/Game/Blueprints/Characters/AI/Melee/BP_Enemy_Melee` OtherActor)))
  (if (`KismetSystemLibrary.IsValid` _movecollision_back)
    (set `PrimitiveComponent.bGenerateOverlapEvents` true _movecollision_back)
    (`self.Push-off` :!label _label_3)
    (goto _label_2 :!via `Stop`)))

(event `self.MoveCollision-back.OnComponentBeginOverlap`
  (params (OverlappedComponent :type "PrimitiveComponent Object Reference") (OtherActor :type "Actor Object Reference") (OtherComp :type "PrimitiveComponent Object Reference") (OtherBodyIndex :type Integer) (bFromSweep :type Boolean) (SweepResult :type "HitResult Structure (by ref)"))
  (cast `/Game/Blueprints/Characters/AI/Shooter/BP_Enemy_Shooter` OtherActor
    (:`then`
      _)
    (:`CastFailed`
      (cast `/Game/Blueprints/Characters/AI/Melee/BP_Enemy_Melee` OtherActor)))
  (set `PrimitiveComponent.bGenerateOverlapEvents` false (`self.MoveCollision-front`))
  (`self.Push-on`)
  (if (`self.Closing`)
    (if (`self.BackSide`)
      (goto _label_2)
      (else
        (goto _label)))
    (else
      (set `self.Closing` (!= (`self.Y-rot`) (`self.Start-Y-rot`)))
      (set `self.BackSide` true)
      (goto _label_2))))

(event `self.MoveCollision-back.OnComponentEndOverlap`
  (params (OverlappedComponent :type "PrimitiveComponent Object Reference") (OtherActor :type "Actor Object Reference") (OtherComp :type "PrimitiveComponent Object Reference") (OtherBodyIndex :type Integer))
  (bind _movecollision_front (`self.MoveCollision-front`))
  (cast `/Game/Blueprints/Characters/AI/Shooter/BP_Enemy_Shooter` OtherActor
    (:`then`
      _)
    (:`CastFailed`
      (cast `/Game/Blueprints/Characters/AI/Melee/BP_Enemy_Melee` OtherActor)))
  (if (`KismetSystemLibrary.IsValid` _movecollision_front)
    (set `PrimitiveComponent.bGenerateOverlapEvents` true _movecollision_front)
    (goto _label_3)))

(event `Push-on`
  (set `PrimitiveComponent.bGenerateOverlapEvents` true (`self.PushBox-back`))
  (set `PrimitiveComponent.bGenerateOverlapEvents` true (`self.PushBox-front`)))

(event `Push-off`
  (set `PrimitiveComponent.bGenerateOverlapEvents` false (`self.PushBox-back`))
  (set `PrimitiveComponent.bGenerateOverlapEvents` false (`self.PushBox-front`)))

(event `self.PushBox-back.OnComponentBeginOverlap`
  (params (OverlappedComponent :type "PrimitiveComponent Object Reference") (OtherActor :type "Actor Object Reference") (OtherComp :type "PrimitiveComponent Object Reference") (OtherBodyIndex :type Integer) (bFromSweep :type Boolean) (SweepResult :type "HitResult Structure (by ref)"))
  (bind _asbp_enemy_shooter (cast `/Game/Blueprints/Characters/AI/Shooter/BP_Enemy_Shooter` OtherActor))
  (bind _output_get (set `self.Knockback-enemy` _asbp_enemy_shooter))
  (set `/Game/Blueprints/Characters/AI/Shooter/BP_Enemy_Shooter.Knockback-rotation` (`KismetMathLibrary.Conv_RotatorToVector` (`KismetMathLibrary.FindLookAtRotation` (`self.K2_GetActorLocation` _output_get) (`SceneComponent.K2_GetComponentLocation` (`self.Center point`)))) _output_get)
  (`/Game/Blueprints/Characters/AI/Shooter/BP_Enemy_Shooter.Door-stun` (`self.Knockback-enemy`)))

(event `self.PushBox-front.OnComponentBeginOverlap`
  (params (OverlappedComponent :type "PrimitiveComponent Object Reference") (OtherActor :type "Actor Object Reference") (OtherComp :type "PrimitiveComponent Object Reference") (OtherBodyIndex :type Integer) (bFromSweep :type Boolean) (SweepResult :type "HitResult Structure (by ref)"))
  (bind _asbp_enemy_shooter (cast `/Game/Blueprints/Characters/AI/Shooter/BP_Enemy_Shooter` OtherActor))
  (bind _output_get (set `self.Knockback-enemy` _asbp_enemy_shooter))
  (set `/Game/Blueprints/Characters/AI/Shooter/BP_Enemy_Shooter.Knockback-rotation` (`KismetMathLibrary.Conv_RotatorToVector` (`KismetMathLibrary.FindLookAtRotation` (`self.K2_GetActorLocation` _output_get) (`SceneComponent.K2_GetComponentLocation` (`self.Center point`)))) _output_get)
  (`/Game/Blueprints/Characters/AI/Shooter/BP_Enemy_Shooter.Door-stun` _asbp_enemy_shooter))

(fn `UserConstructionScript`)