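; A one-shot dialogue trigger box that shows lines from a dialogue asset when BP_Parasite overlaps it, pausing the game.
; On BeginPlay it enables player input and caches the first Dialogue_initiatior actor, whose widget instance displays the text.
; Space advances through the asset's line array while dialogue is active.
; After the last line it hides the widget, unpauses and destroys itself.
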(event `self.ReceiveBeginPlay`
  ;[1 0.3625 0.4122] getting the initiator
  (`self.EnableInput` (`GameplayStatics.GetPlayerController` 0))
  (bind _outactors (`GameplayStatics.GetAllActorsOfClass` "/Game/Blueprints/dialogues/dialogue_initiatior.dialogue_initiatior_C"))
  (set `self.dialogueinitia_var` (`|GetArrayItem` _outactors)))

(event `self.ReceiveActorBeginOverlap`
  (params (OtherActor :type "Actor Object Reference"))
  (bind _widjetinstance (`/Game/Blueprints/dialogues/dialogue_initiatior.widjetinstance` (`self.dialogueinitia_var`)))
  ;[1 0.5837 0.9882] start dialogue
  (cast `/Game/Blueprints/Characters/BP_Parasite` OtherActor)
  (set `self.On-a-dialogue` true)
  (`Widget.SetVisibility` _widjetinstance "Visible")
  (set `/Game/Blueprints/Widgets/textbox.current text` (`|GetArrayItem` (`/Game/Blueprints/dialogues/dialogue_data.dialogue array` (`self.dialogueasset`)) (`self.N.line`)) _widjetinstance)
  (`GameplayStatics.SetGamePaused` true))

(event `Key|SpaceBar` :paused true
  (params (Key :type "Key Structure"))
  (bind _dialogue_array (`/Game/Blueprints/dialogues/dialogue_data.dialogue array` (`self.dialogueasset`)))
  (bind _widjetinstance (`/Game/Blueprints/dialogues/dialogue_initiatior.widjetinstance` (`self.dialogueinitia_var`)))
  ;[1 1 1] continue dialogue
  (:`Pressed`
    (if (`self.On-a-dialogue`)
      (bind _output_get (set `self.N.line` (+ (`self.N.line`) 1)))
      (if (> _output_get (`KismetArrayLibrary.Array_LastIndex` _dialogue_array))
        (`Widget.SetVisibility` _widjetinstance "Hidden")
        (`GameplayStatics.SetGamePaused` false)
        (`self.K2_DestroyActor`)
        (else
          (set `/Game/Blueprints/Widgets/textbox.current text` (`|GetArrayItem` _dialogue_array _output_get) _widjetinstance))))))

(fn `UserConstructionScript`)