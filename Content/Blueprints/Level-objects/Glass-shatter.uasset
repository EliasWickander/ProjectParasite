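; Breakable glass level object that disappears when something overlaps either its front or back trigger box.
; Either overlap immediately destroys the Glass component and both trigger boxes, so neither can fire again.
; The actor then destroys itself after a five-second delay.
; Both overlap events run identical logic, with no filter on which actor triggers them.
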(event `self.TriggerBox-Front.OnComponentBeginOverlap`
  (params (OverlappedComponent :type "PrimitiveComponent Object Reference") (OtherActor :type "Actor Object Reference") (OtherComp :type "PrimitiveComponent Object Reference") (OtherBodyIndex :type Integer) (bFromSweep :type Boolean) (SweepResult :type "HitResult Structure (by ref)"))
  (`ActorComponent.K2_DestroyComponent` (`self.Glass`))
  (`ActorComponent.K2_DestroyComponent` (`self.TriggerBox-Back`))
  (`ActorComponent.K2_DestroyComponent` (`self.TriggerBox-Front`))
  (`|ExecutionSequence`
    (:`then_0`
      (`KismetSystemLibrary.Delay` 5.0)
      (`self.K2_DestroyActor`))))

(event `self.TriggerBox-Back.OnComponentBeginOverlap`
  (params (OverlappedComponent :type "PrimitiveComponent Object Reference") (OtherActor :type "Actor Object Reference") (OtherComp :type "PrimitiveComponent Object Reference") (OtherBodyIndex :type Integer) (bFromSweep :type Boolean) (SweepResult :type "HitResult Structure (by ref)"))
  (`ActorComponent.K2_DestroyComponent` (`self.Glass`))
  (`ActorComponent.K2_DestroyComponent` (`self.TriggerBox-Back`))
  (`ActorComponent.K2_DestroyComponent` (`self.TriggerBox-Front`))
  (`|ExecutionSequence`
    (:`then_0`
      (`KismetSystemLibrary.Delay` 5.0)
      (`self.K2_DestroyActor`))))

(fn `UserConstructionScript`)