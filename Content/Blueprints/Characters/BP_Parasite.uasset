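; Player parasite Blueprint that handles the pause menu and ammo HUD for a character able to possess enemies.
; On BeginPlay it sets Game-and-UI input and creates both widgets, with the pause menu hidden.
; Tick polls the possessed enemy and shows its current ammo only when the equipped weapon is a RangedWeapon.
; TogglePause switches the pause widget's visibility and the game's paused state together.
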(event `self.ReceiveBeginPlay`
  (bind _returnvalue (`GameplayStatics.GetPlayerController` 0))
  (`WidgetBlueprintLibrary.SetInputMode_GameAndUIEx` _returnvalue null "DoNotLock" false)
  (`self.EnableInput` _returnvalue)
  (`|ExecutionSequence`
    (:`then_0`
      (bind _returnvalue_2 (`|CreateWidget` "/Game/Blueprints/Widgets/Pause_Widjet.Pause_Widjet_C"))
      (bind _output_get (set `self.PauseCanvas` _returnvalue_2))
      (`UserWidget.AddToViewport` _returnvalue_2 0)
      (`UserWidget.AddToViewport` _output_get 0)
      (`Widget.SetVisibility` _output_get "Hidden"))
    (:`then_1`
      (bind _returnvalue_3 (`|CreateWidget` "/Game/Blueprints/Widgets/Ammo.Ammo_C"))
      (bind _output_get_2 (set `self.AmmoCanvas` _returnvalue_3))
      (`UserWidget.AddToViewport` _output_get_2 0))))

(event `self.ReceiveTick`
  (params (DeltaSeconds :type "Float (single-precision)"))
  (bind _ammocanvas (`self.AmmoCanvas`))
  (bind _ammocanvas_2 (`self.AmmoCanvas`))
  (`|ExecutionSequence`
    (:`then_0`
      (bind _returnvalue (`self.GetPossessedEnemy`))
      (`/Engine/EditorBlueprintResources/StandardMacros.IsValid` _returnvalue
        (:`Is Valid`
          (`Widget.SetVisibility` _ammocanvas "Visible")
          (bind _asranged_weapon (cast `RangedWeapon` (`PawnEnemy.equippedWeapon` _returnvalue))
            (:`then`
              (`/Game/Blueprints/Widgets/Ammo.Ammotext` _ammocanvas_2 (`RangedWeapon.currentAmmo` _asranged_weapon)))
            (:`CastFailed`
              (`Widget.SetVisibility` _ammocanvas_2 "Hidden"))))
        (:`Is Not Valid`
          (`Widget.SetVisibility` _ammocanvas "Hidden"))))))

(fn `TogglePause`
  (params (Enabled :type Boolean))
  (bind _pausecanvas (`self.PauseCanvas`))
  (if Enabled
    (`Widget.SetVisibility` _pausecanvas "Visible")
    (`GameplayStatics.SetGamePaused` true)
    (else
      (`Widget.SetVisibility` _pausecanvas "Hidden")
      (`GameplayStatics.SetGamePaused` false))))

(fn `UserConstructionScript`)