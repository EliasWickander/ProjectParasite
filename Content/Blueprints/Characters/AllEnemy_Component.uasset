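; Shared component for melee and shooter enemies, handling weapon pickup and throwing, knockback, stun and attack camera shakes.
; It caches its owner on BeginPlay, and most events branch on an enemy type enum.
; Throwing replaces the equipped knife or pistol with a thrown-weapon actor carrying mesh and ammo.
; Knockback hits only unpossessed enemies, stunning them via AI controller state and pushing them away through a Delay-driven movement-input loop.
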(event `self.ReceiveBeginPlay`
  (bind _returnvalue (`self.GetOwner`))
  ;[1 1 1] On start
  (bind _asbp_enemy_melee (cast `/Game/Blueprints/Characters/AI/Melee/BP_Enemy_Melee` _returnvalue)
    (:`then`
      (bind _output_get (set `self.Melee` _asbp_enemy_melee))
      (set `self.ParentActor` _output_get))
    (:`CastFailed`
      (bind _asbp_enemy_shooter (cast `/Game/Blueprints/Characters/AI/Shooter/BP_Enemy_Shooter` _returnvalue))
      (bind _output_get_2 (set `self.Shooter` _asbp_enemy_shooter))
      (set `self.ParentActor` _output_get_2))))

(event `Pick up weapon`
  ;[1 1 1] Pick up weapon
  (`self.WeaponPikcup` (`self.Shooter`) (`self.Melee`) (`self.Enemy-type`)))

(event `Weapon-throw`
  (bind _weapon_type_enum (`self.Weapon-Type-enum`))
  (bind _weapon_type_enum_2 (`self.Weapon-Type-enum`))
  ;[1 1 1] Weapon throw
  (`self.Set weapon`)
  (switch `/Game/Blueprints/Characters/EnemyEnum` (`self.Enemy-type`)
    (:`NewEnumerator0`
      (`|ExecutionSequence`
        (:`then_0`
          (bind _asranged_weapon (cast `RangedWeapon` (`PawnEnemy.equippedWeapon` (`self.Melee`))))
          (set `self.Gun-ammo` (`RangedWeapon.currentAmmo` _asranged_weapon)))
        (:`then_1`
          (`Actor.K2_DestroyActor` (`PawnEnemy.equippedWeapon` (`self.Melee`)))
          (`PawnEnemy.SetWeapon` (`self.Melee`) null)
          (bind _returnvalue (`|SpawnActorFromClass` "/Game/Blueprints/Projectiles/WeaponThrow_base_bp.WeaponThrow_base_bp_C" (`Actor.GetTransform` (`self.GetOwner`)) "Undefined" "OverrideRootScale" null null))
          (bind _weaponvisual (`/Game/Blueprints/Projectiles/WeaponThrow_base_bp.WeaponVisual` _returnvalue))
          (`StaticMeshComponent.SetStaticMesh` _weaponvisual (`self.Weapon-all-visual`))
          (set `/Game/Blueprints/Projectiles/WeaponThrow_base_bp.ThrowingWeaponEnum` _weapon_type_enum _returnvalue)
          (set `/Game/Blueprints/Projectiles/WeaponThrow_base_bp.Ammo` (`self.Gun-ammo`) _returnvalue)
          (switch `/Game/Blueprints/Weapons/WeaponEnum` _weapon_type_enum
            (:`NewEnumerator0`
              (`PrimitiveComponent.SetMaterial` _weaponvisual 0 (`self.Knife-mat`)))
            (:`NewEnumerator1`
              (`PrimitiveComponent.SetMaterial` _weaponvisual 0 (`self.Gun-mat`)))))))
    (:`NewEnumerator1`
      (`|ExecutionSequence`
        (:`then_0`
          (bind _asranged_weapon_2 (cast `RangedWeapon` (`PawnEnemy.equippedWeapon` (`self.Shooter`))))
          (set `self.Gun-ammo` (`RangedWeapon.currentAmmo` _asranged_weapon_2)))
        (:`then_1`
          (`Actor.K2_DestroyActor` (`PawnEnemy.equippedWeapon` (`self.Shooter`)))
          (`PawnEnemy.SetWeapon` (`self.Shooter`) null)
          (bind _returnvalue_2 (`|SpawnActorFromClass` "/Game/Blueprints/Projectiles/WeaponThrow_base_bp.WeaponThrow_base_bp_C" (`Actor.GetTransform` (`self.GetOwner`)) "Undefined" "OverrideRootScale" null null))
          (bind _weaponvisual_2 (`/Game/Blueprints/Projectiles/WeaponThrow_base_bp.WeaponVisual` _returnvalue_2))
          (`StaticMeshComponent.SetStaticMesh` _weaponvisual_2 (`self.Weapon-all-visual`))
          (set `/Game/Blueprints/Projectiles/WeaponThrow_base_bp.ThrowingWeaponEnum` _weapon_type_enum_2 _returnvalue_2)
          (set `/Game/Blueprints/Projectiles/WeaponThrow_base_bp.Ammo` (`self.Gun-ammo`) _returnvalue_2)
          (switch `/Game/Blueprints/Weapons/WeaponEnum` _weapon_type_enum_2
            (:`NewEnumerator0`
              (`PrimitiveComponent.SetMaterial` _weaponvisual_2 0 (`self.Knife-mat`)))
            (:`NewEnumerator1`
              (`PrimitiveComponent.SetMaterial` _weaponvisual_2 0 (`self.Gun-mat`)))))))))

(event `Set weapon`
  (bind _equippedweapon (`PawnEnemy.equippedWeapon` (`self.Shooter`)))
  (bind _equippedweapon_2 (`PawnEnemy.equippedWeapon` (`self.Melee`)))
  ;[1 1 1] Set weapon
  (switch `/Game/Blueprints/Characters/EnemyEnum` (`self.Enemy-type`)
    (:`NewEnumerator0`
      ;;[1 1 1] These are causing the error
      (cast `/Game/Blueprints/Weapons/BP_Knife` _equippedweapon_2
        (:`then`
          (set `self.Weapon-Type-enum` "NewEnumerator0" :!label _label))
        (:`CastFailed`
          (cast `/Game/Blueprints/Weapons/BP_Pistol` _equippedweapon_2)
          (set `self.Weapon-Type-enum` "NewEnumerator1" :!label _label_2))))
    (:`NewEnumerator1`
      (cast `/Game/Blueprints/Weapons/BP_Knife` _equippedweapon
        (:`then`
          (goto _label))
        (:`CastFailed`
          (cast `/Game/Blueprints/Weapons/BP_Pistol` _equippedweapon)
          (goto _label_2))))))

(event `EnemyKnockback`
  (bind (_returnvalue_x _returnvalue_y _returnvalue_z) (`KismetMathLibrary.BreakVector` (* (`KismetMathLibrary.Conv_RotatorToVector` (`KismetMathLibrary.FindLookAtRotation` (`Actor.K2_GetActorLocation` (`self.ParentActor`)) (`self.KnockbackVector`))) -1.0)))
  ;[1 1 1] Knockback
  (switch `/Game/Blueprints/Characters/EnemyEnum` (`self.Enemy-type`)
    (:`NewEnumerator0`
      (if (not (`PawnEnemy.isPossessed` (`self.Melee`)))
        (`self.EnemyStun-all` :!label _label_3)
        (`KismetSystemLibrary.PrintString` "Knockback is reached")
        (bind _output_get (set `self.KnockbackTimer` 15))
        (if (<= 0 _output_get) :!label _label_4
          (`|ExecutionSequence`
            (:`then_0`
              (set `self.KnockbackTimer` (- (`self.KnockbackTimer`) 1))
              (`KismetSystemLibrary.Delay` 0.016)
              (goto _label_4))
            (:`then_1`
              (`Pawn.AddMovementInput` (`Actor.Instigator` (`self.ParentActor`)) (`KismetMathLibrary.MakeVector` _returnvalue_x 0.0 _returnvalue_z) 1.0 true)
              (if (<= (`self.KnockbackTimer`) 0)
                (`KismetSystemLibrary.Delay` 0.2)
                (set `self.KnockbackTimer` 15)))))))
    (:`NewEnumerator1`
      (if (not (`PawnEnemy.isPossessed` (`self.Shooter`)))
        (goto _label_3)))))

(event `EnemyStun-all`
  (bind _returnvalue (`self.GetOwner`))
  ;[1 1 1] Stun
  (switch `/Game/Blueprints/Characters/EnemyEnum` (`self.Enemy-type`)
    (:`NewEnumerator0`
      (bind _asmelee_aicontroller (cast `MeleeAIController` (`AIBlueprintHelperLibrary.GetAIController` (`self.GetOwner`))))
      (`AIControllerBase.SetCurrentState` _asmelee_aicontroller "State_Stunned")
      (`KismetSystemLibrary.Delay` (`self.StunTime`))
      (`AIControllerBase.SetCurrentState` _asmelee_aicontroller "State_Chase"))
    (:`NewEnumerator1`
      (bind _asshooter_aicontroller (cast `ShooterAIController` (`AIBlueprintHelperLibrary.GetAIController` _returnvalue)))
      (bind _asbp_enemy_shooter (cast `/Game/Blueprints/Characters/AI/Shooter/BP_Enemy_Shooter` _returnvalue))
      (`AIControllerBase.SetCurrentState` _asshooter_aicontroller "State_Stunned")
      (bind _spinningstarsactor (`/Game/Blueprints/Characters/AI/Shooter/BP_Enemy_Shooter.SpinningStarsActor` _asbp_enemy_shooter))
      (`ChildActorComponent.SetChildActorClass` _spinningstarsactor "/Game/Art/Particles/Spinning_Star/BP_SpinningStars.BP_SpinningStars_C")
      (`KismetSystemLibrary.Delay` (`self.StunTime`))
      (`ChildActorComponent.SetChildActorClass` _spinningstarsactor null)
      (`AIControllerBase.SetCurrentState` _asshooter_aicontroller "State_Chase")))
  (`KismetSystemLibrary.PrintString` "unstunned"))

(event `ShootingScreenshake`
  ;[1 1 1] Scerenshakes
  (`|ExecutionSequence`
    (:`then_0`
      (`self.Set weapon`))
    (:`then_1`
      (switch `/Game/Blueprints/Weapons/WeaponEnum` (`self.Weapon-Type-enum`)
        (:`NewEnumerator0`
          (if (not (`self.GunShakeCooldown`))
            (`PlayerController.ClientStartCameraShake` :`self` (`GameplayStatics.GetPlayerController` 0) :`Shake` "/Game/Blueprints/PlayerControllers/KnifeSlash.KnifeSlash_C")
            (set `self.GunShakeCooldown` true)
            (`KismetSystemLibrary.Delay` 0.8)
            (set `self.GunShakeCooldown` false)))
        (:`NewEnumerator1`
          (if (not (`self.GunShakeCooldown`))
            (switch `/Game/Blueprints/Characters/EnemyEnum` (`self.Enemy-type`)
              (:`NewEnumerator0`
                ;[1 1 1] Check if ammo then shake
                (bind _asranged_weapon (cast `RangedWeapon` (`PawnEnemy.equippedWeapon` (`self.Melee`))))
                (if (not (== (`RangedWeapon.currentAmmo` _asranged_weapon) 0))
                  (`PlayerController.ClientStartCameraShake` :`self` (`GameplayStatics.GetPlayerController` 0) :`Shake` "/Game/Blueprints/PlayerControllers/HandGunShake.HandGunShake_C" :!label _label_5)
                  (set `self.GunShakeCooldown` true)
                  (`KismetSystemLibrary.Delay` 0.015)
                  (set `self.GunShakeCooldown` false)))
              (:`NewEnumerator1`
                (bind _asranged_weapon_2 (cast `RangedWeapon` (`PawnEnemy.equippedWeapon` (`self.Shooter`))))
                (if (not (== (`RangedWeapon.currentAmmo` _asranged_weapon_2) 0))
                  (goto _label_5))))))))))

(fn `WeaponPikcup`
  (params (PossessedShooter :type "/Game/Blueprints/Characters/AI/Shooter/BP_Enemy_Shooter Object Reference") (PossessedMelee :type "/Game/Blueprints/Characters/AI/Melee/BP_Enemy_Melee Object Reference") (`What enemy` :type "/Game/Blueprints/Characters/EnemyEnum Enum" :default "NewEnumerator0"))
  (locals (`Weapon var` :type "WeaponBase Object Reference"))
  (switch `/Game/Blueprints/Characters/EnemyEnum` `What enemy`
    (:`NewEnumerator0`
      (for _array_element (`Actor.GetOverlappingActors` (`self.GetOwner`) "/Script/ProjectParasite.WeaponBase")
        (bind _asweapon_base (cast `WeaponBase` _array_element))
        (bind _output_get (set `local.Weapon var` _asweapon_base))
        (if (not (`WeaponBase.isEquipped` _output_get))
          (`PawnEnemy.SetWeapon` PossessedMelee (`local.Weapon var`)))))
    (:`NewEnumerator1`
      (for _array_element_2 (`Actor.GetOverlappingActors` (`self.GetOwner`) "/Script/ProjectParasite.WeaponBase")
        (bind _asweapon_base_2 (cast `WeaponBase` _array_element_2))
        (bind _output_get_2 (set `local.Weapon var` _asweapon_base_2))
        (if (not (`WeaponBase.isEquipped` _output_get_2))
          (`PawnEnemy.SetWeapon` PossessedShooter (`local.Weapon var`)))))))