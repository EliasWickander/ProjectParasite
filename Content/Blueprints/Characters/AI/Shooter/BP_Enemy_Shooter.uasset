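; Shooter enemy AI character Blueprint, whose live graph logic mainly handles blood-style splatter when damaged.
; OnDamagedbyCharacter spawns a particle emitter whose collisions print a debug string and place temporary decals, randomly sized, with a random material frame.
; PickupWeapon equips overlapping unequipped weapons, but its graph call is disconnected.
; Blackboard setup, stun states, knockback timeline and weapon throwing are also unwired, leaving their events empty.
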(event `self.ReceiveBeginPlay`)

(event `self.OnDamagedByCharacter`
  (bind _returnvalue (`GameplayStatics.SpawnEmitterAtLocation` "/Game/placeholders_contente/placeholder_vfx1/splatter_P.splatter_P" (`self.K2_GetActorLocation`)))
  (add `ParticleSystemComponent.OnParticleCollide` _returnvalue (delegate `on_coll2`)))

(event `WPNthrow`)

(event `on_coll2`
  (params (EventName :type Name) (EmitterTime :type "Float (double-precision)") (ParticleTime :type Integer) (Location :type "Vector Structure") (Velocity :type "Vector Structure") (Direction :type "Vector Structure") (Normal :type "Vector Structure") (BoneName :type Name) (PhysMat :type "PhysicalMaterial Object Reference"))
  (`KismetSystemLibrary.PrintString` "Hello")
  (bind _returnvalue (`KismetMaterialLibrary.CreateDynamicMaterialInstance` "/Game/placeholders_contente/placeholder_vfx1/Splatter_decal.Splatter_decal"))
  (`MaterialInstanceDynamic.SetScalarParameterValue` _returnvalue "Frame" (`KismetMathLibrary.Conv_IntToDouble` (`KismetMathLibrary.RandomInteger` 11)))
  (`GameplayStatics.SpawnDecalAtLocation` _returnvalue (`KismetMathLibrary.Conv_DoubleToVector` (`KismetMathLibrary.RandomFloatInRange` 30.0 50.0)) Location (`KismetMathLibrary.Conv_VectorToRotator` Normal) 30.0))

(event `Stunning`)

(event `Door-stun`)

(event `InputAction|Interact`
  (params (Key :type "Key Structure")))

(fn `Pickup Weapon`
  (locals (LoopedWeapon :type "WeaponBase Object Reference"))
  (for _array_element (`self.GetOverlappingActors` "/Script/ProjectParasite.WeaponBase")
    (bind _asweapon_base (cast `WeaponBase` _array_element))
    (bind _output_get (set `local.LoopedWeapon` _asweapon_base))
    (if (not (`WeaponBase.isEquipped` _output_get))
      (`self.SetWeapon` (`local.LoopedWeapon`)))))

(fn `UserConstructionScript`)