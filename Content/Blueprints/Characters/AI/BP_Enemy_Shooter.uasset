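; BP_Enemy_Shooter is a shooter enemy character whose ShooterAIController and blackboard state switch between stun and chase.
; PermaStun sets the controller's stun state at BeginPlay; Door-stun triggers a three-second blackboard stun plus timeline-scaled knockback through forced movement input.
; WPNthrow spawns a throwable using the weapon's mesh when allowed.
; An Interact input equips overlapping unequipped weapons through PickupWeapon.
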(event `self.ReceiveBeginPlay`
  (if (`self.PermaStun`)
    (bind _asshooter_aicontroller (cast `ShooterAIController` (`AIBlueprintHelperLibrary.GetAIController` null)))
    (set `ShooterAIController.currentState` (`self.Stun-state`) _asshooter_aicontroller)))

(event `WPNthrow`
  (if (`self.CanThrow`)
    (bind _returnvalue (`|SpawnActorFromClass` "/Game/Blueprints/Projectiles/WeaponThrow_base_bp.WeaponThrow_base_bp_C" (`self.GetTransform`) "Undefined" "OverrideRootScale" null null))
    (`StaticMeshComponent.SetStaticMesh` (`/Game/Blueprints/Projectiles/WeaponThrow_base_bp.WeaponVisual` _returnvalue) (`self.WeaponVisual`))))

(event `Stunning`
  (`BlackboardComponent.SetValueAsEnum` (`AIBlueprintHelperLibrary.GetBlackboard` null) (`KismetStringLibrary.Conv_StringToName` "CurrentState") (`self.Stun-state`))
  (`KismetSystemLibrary.Delay` 3.0)
  (`BlackboardComponent.SetValueAsEnum` (`AIBlueprintHelperLibrary.GetBlackboard` null) (`KismetStringLibrary.Conv_StringToName` "CurrentState") (`self.Chase-state`)))

(event `Door-stun`
  (bind (_returnvalue_x _returnvalue_y _returnvalue_z) (`KismetMathLibrary.BreakVector` (* (`self.Knockback-rotation`) -1.0)))
  (cast `ShooterAIController` (`self.GetController`))
  (`self.Stunning`)
  ;[1 1 1] Knockback direction
  (bind (_direction _knockbackscale) (`Timeline|Knockback timeline` :!via `PlayFromStart`)
    (:`Update`
      (`self.AddMovementInput` (`KismetMathLibrary.MakeVector` _returnvalue_x 0.0 _returnvalue_z) _knockbackscale true))))

(event `InputAction|Interact`
  (params (Key :type "Key Structure"))
  (:`Pressed`
    (`self.PickupWeapon`)))

(fn `PickupWeapon`
  (locals (LoopedWeapon :type "WeaponBase Object Reference"))
  (for _array_element (`self.GetOverlappingActors` "/Script/ProjectParasite.WeaponBase")
    (bind _asweapon_base (cast `WeaponBase` _array_element))
    (bind _output_get (set `local.LoopedWeapon` _asweapon_base))
    (if (not (`WeaponBase.isEquipped` _output_get))
      (`self.SetWeapon` (`local.LoopedWeapon`)))))

(fn `UserConstructionScript`)