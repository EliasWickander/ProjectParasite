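; Melee enemy character that can be possessed, handling possession visuals and blood splatter on damage.
; BeginPlay sets the enemy type, caches the post-process Blueprint and creates a dynamic possessed material.
; Possession triggers the post-process blur while a timeline animates the material's CP1 parameter.
; Damage spawns a splatter emitter whose particle collisions place randomly framed, sized decals; stun logic is disconnected and MeleeThrow is empty.
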(event `Stunning-melee`
  ;[1 1 1] Outdated
)

(event `self.ReceiveBeginPlay`
  (set `/Game/Blueprints/Characters/AllEnemy_Component.Enemy-type` "NewEnumerator0" (`self.RegretfullChild`))
  (bind _outactors (`GameplayStatics.GetAllActorsOfClass` "/Game/Blueprints/Level-objects/postProcess_Blueprint.postProcess_Blueprint_C"))
  (bind _aspost_process_blueprint (cast `/Game/Blueprints/Level-objects/postProcess_Blueprint` (`|GetArrayItem` _outactors))
    (:`then`
      (set `self.PPP` _aspost_process_blueprint)
      (bind _returnvalue (`PrimitiveComponent.CreateDynamicMaterialInstance` (`self.skeletalMesh`) 1 "/Game/Art/Materials/OirigianlsLinus/EnemyOnePossesed_Mat.EnemyOnePossesed_Mat" "None"))
      (set `self.PORCODDIOMAT` _returnvalue))
    (:`CastFailed`
      (`KismetSystemLibrary.PrintString` "NO POSTPROCESSPROFILE"))))

(event `MeleeThrow`
  ;[1 1 1] Outdated
)

(event `self.OnPossessed`
  ;[1 1 1] Blur on possess
  (`|ExecutionSequence`
    (:`then_0`
      (`/Game/Blueprints/Level-objects/postProcess_Blueprint.Blurthis` (`self.PPP`)))
    (:`then_1`
      (bind (_direction _shaderchange) (`Timeline|Timeline_0` :!via `PlayFromStart`)
        (:`Update`
          (`MaterialInstanceDynamic.SetScalarParameterValue` (`self.PORCODDIOMAT`) "CP1" _shaderchange))))))

(event `self.OnDamagedByCharacter`
  (bind _returnvalue (`GameplayStatics.SpawnEmitterAtLocation` "/Game/placeholders_contente/placeholder_vfx1/splatter_P.splatter_P" (`self.K2_GetActorLocation`)))
  (add `ParticleSystemComponent.OnParticleCollide` _returnvalue (delegate `on_coll2`)))

(event `on_coll2`
  (params (EventName :type Name) (EmitterTime :type "Float (double-precision)") (ParticleTime :type Integer) (Location :type "Vector Structure") (Velocity :type "Vector Structure") (Direction :type "Vector Structure") (Normal :type "Vector Structure") (BoneName :type Name) (PhysMat :type "PhysicalMaterial Object Reference"))
  (bind _returnvalue (`KismetMaterialLibrary.CreateDynamicMaterialInstance` "/Game/placeholders_contente/placeholder_vfx1/Splatter_decal.Splatter_decal"))
  (`MaterialInstanceDynamic.SetScalarParameterValue` _returnvalue "Frame" (`KismetMathLibrary.Conv_IntToDouble` (`KismetMathLibrary.RandomInteger` 11)))
  (`GameplayStatics.SpawnDecalAtLocation` _returnvalue (`KismetMathLibrary.Conv_DoubleToVector` (`KismetMathLibrary.RandomFloatInRange` 30.0 50.0)) Location (`KismetMathLibrary.Conv_VectorToRotator` Normal) 30.0))

(fn `UserConstructionScript`)