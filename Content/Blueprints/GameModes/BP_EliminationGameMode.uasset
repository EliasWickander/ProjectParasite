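; BP_EliminationGameMode is a game mode that handles two outcomes: a finished floor and the player's death.
; OnFloorFinished shows the Level_Clear widget and spawns the NS_Staircase Niagara effect at the first BP_GoalTrigger found in the level.
; OnPlayerDied shows the Lose_widjet screen, pauses the game and stores the pause call's result in IsGameLost.
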(event `self.OnFloorFinished`
  (bind _returnvalue (`|CreateWidget` "/Game/Blueprints/Widgets/Level_Clear.Level_Clear_C"))
  (`UserWidget.AddToViewport` _returnvalue 0)
  (bind _outactors (`GameplayStatics.GetAllActorsOfClass` "/Game/Blueprints/BP_GoalTrigger.BP_GoalTrigger_C"))
  (`NiagaraFunctionLibrary.SpawnSystemAtLocation` "/Game/Art/Particles/Staircase/NS_Staircase.NS_Staircase" (`self.K2_GetActorLocation` (`|GetArrayItem` _outactors))))

(event `self.OnPlayerDied`
  (bind _returnvalue (`|CreateWidget` "/Game/Blueprints/Widgets/lose_widjet.lose_widjet_C"))
  (`UserWidget.AddToViewport` _returnvalue 0)
  (bind _returnvalue_2 (`GameplayStatics.SetGamePaused` true))
  (set `self.IsGameLost` _returnvalue_2))

(fn `UserConstructionScript`)