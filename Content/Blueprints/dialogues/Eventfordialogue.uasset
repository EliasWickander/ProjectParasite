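; Dialogue controller actor that plays a dialogue asset line by line in a shared widget while the game is paused.
; On BeginPlay it enables player input and caches the first Dialogue_initiatior actor, which holds the widget.
; Fromdialogue stores the passed asset, shows its first line and pauses the game.
; SpaceBar advances the line, hiding the widget and unpausing after the last, though Onadialogue is never cleared.
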(event `self.ReceiveBeginPlay`
  (`self.EnableInput` (`GameplayStatics.GetPlayerController` 0))
  (bind _outactors (`GameplayStatics.GetAllActorsOfClass` "/Game/Blueprints/dialogues/dialogue_initiatior.dialogue_initiatior_C"))
  (set `self.dialogueinitia_var` (`|GetArrayItem` _outactors)))

(event `Key|SpaceBar` :paused true
  (params (Key :type "Key Structure"))
  (bind _dialogue_array (`/Game/Blueprints/dialogues/dialogue_data.dialogue array` (`self.dialogueasset`)))
  (bind _widjetinstance (`/Game/Blueprints/dialogues/dialogue_initiatior.widjetinstance` (`self.dialogueinitia_var`)))
  (:`Pressed`
    (if (`self.On-a-dialogue`)
      (bind _output_get (set `self.N.line` (+ (`self.N.line`) 1)))
      (if (> _output_get (`KismetArrayLibrary.Array_LastIndex` _dialogue_array))
        (`Widget.SetVisibility` _widjetinstance "Hidden")
        (`GameplayStatics.SetGamePaused` false)
        (else
          (set `/Game/placeholders_contente/test_widget/textbox.current text` (`|GetArrayItem` _dialogue_array _output_get) _widjetinstance))))))

(fn `fromdialogue`
  (params (customDialogue :type "/Game/Blueprints/dialogues/dialogue_data Object Reference"))
  (bind _widjetinstance (`/Game/Blueprints/dialogues/dialogue_initiatior.widjetinstance` (`self.dialogueinitia_var`)))
  (set `self.On-a-dialogue` true)
  (set `self.N.line` 0)
  (set `self.Dialogueasset` customDialogue)
  (`Widget.SetVisibility` _widjetinstance "Visible")
  (set `/Game/placeholders_contente/test_widget/textbox.current text` (`|GetArrayItem` (`/Game/Blueprints/dialogues/dialogue_data.dialogue array` (`self.Dialogueasset`)) (`self.N.line`)) _widjetinstance)
  (`GameplayStatics.SetGamePaused` true))

(fn `UserConstructionScript`)