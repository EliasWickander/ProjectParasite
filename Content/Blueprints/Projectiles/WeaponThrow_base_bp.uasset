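; Base projectile for a thrown weapon that stuns BP_Enemy_Shooter enemies on contact.
; It attaches a Niagara trail at BeginPlay and rotates the weapon visual each tick while in flight.
; The first valid overlap removes the projectile movement, stops the spin shortly after, and destroys the actor after a delay.
; Weapon pickup and the ground-spawn event are unimplemented placeholders.
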(event `self.ReceiveBeginPlay`
  (`NiagaraFunctionLibrary.SpawnSystemAttached` "/Game/Art/Particles/Throw_trail-NS.Throw_trail-NS" (`self.WeaponVisual`) "None" (0.0 0.0 0.0) (struct) "KeepRelativeOffset"))

(event `self.ReceiveTick`
  (params (DeltaSeconds :type "Float (single-precision)"))
  (if (`self.ded`)
    _
    (elif (`self.IsSpeeeen`)
      (`SceneComponent.K2_AddWorldRotation` (`self.WeaponVisual`) (struct :`Yaw` 5.0) false false))))

(event `self.WeaponCollision.OnComponentBeginOverlap`
  (params (OverlappedComponent :type "PrimitiveComponent Object Reference") (OtherActor :type "Actor Object Reference") (OtherComp :type "PrimitiveComponent Object Reference") (OtherBodyIndex :type Integer) (bFromSweep :type Boolean) (SweepResult :type "HitResult Structure (by ref)"))
  (bind _projectilemovement (`self.ProjectileMovement`))
  (set `self.Other Actor` OtherActor)
  (if (`KismetSystemLibrary.IsValid` _projectilemovement)
    (`|ExecutionSequence`
      (:`then_0`
        (`KismetSystemLibrary.Delay` 0.1)
        (set `self.IsSpeeeen` false))
      (:`then_1`
        (`ActorComponent.K2_DestroyComponent` _projectilemovement)
        (bind _asbp_enemy_shooter (cast `/Game/AI/Shooter/BP_Enemy_Shooter` (`self.Other Actor`))
          (:`then`
            (`/Game/AI/Shooter/BP_Enemy_Shooter.Stunning` _asbp_enemy_shooter))
          (:`CastFailed`
            (`KismetSystemLibrary.PrintString` "Not enemy"))))
      (:`then_2`
        ;[1 1 1] Add weapon pickup later
        (`KismetSystemLibrary.Delay` 3.0)
        (`self.K2_DestroyActor`)))))

(event `ThrownWPN-spawn`
  ;[1 1 1] Make the thrown weapon appear on the ground
)

(fn `UserConstructionScript`)