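; Player controller that handles gated tutorial actions and weapon throwing for the possessed pawn.
; A Tutorial-player event enables tutorial mode, where Fire or Possess, when its flag is set, unpauses the game, clears the flag and triggers the shooter's Attack or the parasite's Dash.
; Throw calls WPNthrow on a shooter pawn regardless of tutorial state; its separate tutorial check leads to no action.
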(event `Tutorial-player`
  (set `self.IsTutorial` true))

(event `InputAction|Fire` :paused true
  (params (Key :type "Key Structure"))
  (:`Pressed`
    (if (`self.IsTutorial`)
      (if (`self.Fire-tutorial`)
        (`GameplayStatics.SetGamePaused` false)
        (set `self.Fire-tutorial` false)
        (bind _asbp_enemy_shooter (cast `/Game/AI/Shooter/BP_Enemy_Shooter` (`GameplayStatics.GetPlayerPawn` 0)))
        (`PawnEnemyRanged.Attack` _asbp_enemy_shooter)))))

(event `InputAction|Possess` :paused true
  (params (Key :type "Key Structure"))
  (:`Pressed`
    (if (`self.IsTutorial`)
      (if (`self.Possession-tutorial`)
        (`GameplayStatics.SetGamePaused` false)
        (set `self.Possession-tutorial` false)
        (bind _asbp_parasite (cast `/Game/Blueprints/Characters/BP_Parasite` (`GameplayStatics.GetPlayerPawn` 0)))
        (bind _output_get (set `self.As BP Parasite` _asbp_parasite))
        (`PawnParasite.Dash` _output_get)))))

(event `InputAction|Throw` :paused true
  (params (Key :type "Key Structure"))
  (:`Pressed`
    (if (`self.IsTutorial`)
      (if (`self.Throwing-tutorial`)
        _))))

(event `InputAction|Throw`
  (params (Key :type "Key Structure"))
  (:`Pressed`
    (bind _asbp_enemy_shooter (cast `/Game/AI/Shooter/BP_Enemy_Shooter` (`GameplayStatics.GetPlayerPawn` 0))
      (:`then`
        (`/Game/AI/Shooter/BP_Enemy_Shooter.WPNthrow` _asbp_enemy_shooter))
      (:`CastFailed`
        (`KismetSystemLibrary.PrintString` "Not found")))))

(fn `UserConstructionScript`)